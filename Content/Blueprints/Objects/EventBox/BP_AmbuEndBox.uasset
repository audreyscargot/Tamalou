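; BP_AmbuEndBox is an event box with a box collision that shows countdown and win screens, apparently marking an end point.
; End-overlap events are forwarded to OnOverlapEnd, whose logic is not in these graphs.
; ShowTempFeedback adds or removes a three-count countdown widget, marked as temporary, and EndFunction displays a temporary win widget.
; A timer-clearing node is left unconnected and never runs.
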(event OnComponentEndOverlap(BoxCollision)
  (params (OverlappedComponent :type Primitive%20Component%20Object%20Reference) (OtherActor :type Actor%20Object%20Reference) (OtherComp :type Primitive%20Component%20Object%20Reference) (OtherBodyIndex :type Integer))
  (Class|AmbulanceEndBox|OnOverlapEnd OverlappedComponent OtherActor OtherComp OtherBodyIndex))

(event EventShowTempFeedback
  (params (_yes :type Boolean))
  ;[0.15 0.15 0.15 0.5] TEMPORAIRE
  (if _yes
    (bind _returnvalue (UserInterface|CreateWidget "/Game/DebugWidgets/TEMPWBP_Countdown.TEMPWBP_Countdown_C" 0 3))
    (bind _output_get (Variables|Default|SetTEMPFeedback _returnvalue))
    (UserInterface|Viewport|AddtoViewport _output_get 0)
    (else
      (Widget|RemovefromParent (Variables|Default|GetTEMPFeedback)))))

(event EventEndFunction
  ;[0.15 0.15 0.15 0.5] TEMPORAIRE
  (bind _returnvalue (UserInterface|CreateWidget "/Game/DebugWidgets/TEMPWBP_Win.TEMPWBP_Win_C"))
  (UserInterface|Viewport|AddtoViewport _returnvalue 0))

(fn ConstructionScript)