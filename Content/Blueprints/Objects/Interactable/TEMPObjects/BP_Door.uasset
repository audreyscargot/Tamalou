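; BP_Door is a temporary interactable door that swings its static mesh around yaw when OpenDoor is called.
; BeginPlay caches the mesh's starting rotation, and OpenDoor toggles DoorIsOpen to play or reverse one timeline.
; The timeline lerps yaw up to 90 degrees from that start, using a separate locked alpha track when IsLocked is set.
; The open flag toggles even while locked.
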(event EventOpenDoor
  (bind _ogrot (Variables|Default|GetOGRot))
  (bind (_roll _pitch _yaw) (Math|Rotator|BreakRotator _ogrot))
  (if (Variables|Default|GetDoorIsOpen)
    (Variables|Default|SetDoorIsOpen false)
    (bind (_direction _alphaopen _alphalocked) (Timeline|OpenDoorTimeline Reverse)
      (:Update
        (Transformation|SetWorldRotation (Variables|Default|GetStaticMesh) (Math|Rotator|MakeRotator _roll _pitch (Math|Float|Lerp _yaw (+ _yaw 9e+01) (Math|Float|SelectFloat _alphaopen _alphalocked (not (Variables|Default|GetIsLocked))))) false false)))
    (else
      (Variables|Default|SetDoorIsOpen true)
      (Timeline|OpenDoorTimeline Play))))

(event EventBeginPlay
  (Variables|Default|SetOGRot (Transformation|GetWorldRotation (Variables|Default|GetStaticMesh))))

(fn ConstructionScript)