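; BP_PlayerCharacter is the player character Blueprint, and its event graph holds only debug key handlers.
; The T handler, marked TEMP, teleports a BP_SaveableNPC to the player and grabs its mesh with HandleComponent.
; Before the grab, it sets the player capsule to ignore PhysicsBody collisions.
; Tab calls QuickReload, Escape quits the game, and the construction script is empty.
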(event Input|KeyboardEvents|DebugKeyTab
  (params (Key :type Key%20Structure :default "None") (ActionValue :type Input%20Action%20Value%20Structure))
  ;[0.15 0.15 0.15 0.5] TEMP
  (:Pressed
    (Class|PlayerCharacter|QuickReload)))

(event Input|KeyboardEvents|DebugKeyT
  (params (Key :type Key%20Structure :default "None") (ActionValue :type Input%20Action%20Value%20Structure))
  ;[0.15 0.15 0.15 0.5] TEMP
  (:Pressed
    (bind _returnvalue (Actor|GetActorOfClass "/Game/Blueprints/Objects/NPC/BP_SaveableNPC.BP_SaveableNPC_C"))
    (Collision|SetCollisionResponsetoChannel (Variables|Default|GetCapsuleComponent) "ECC_PhysicsBody" "ECR_Ignore")
    (Transformation|SetActorLocation _returnvalue (Transformation|GetActorLocation) false true)
    (Physics|Components|PhysicsHandle|GrabComponentatLocationwithRotation (Variables|Default|GetHandleComponent) (Variables|/Script/Engine.Character|GetMesh _returnvalue) "None" (Transformation|GetActorLocation) "0, 0, 0")))

(event Input|KeyboardEvents|DebugKeyEscape
  (params (Key :type Key%20Structure :default "None") (ActionValue :type Input%20Action%20Value%20Structure))
  ;[0.15 0.15 0.15 0.5] TEMP
  (:Pressed
    (Game|QuitGame 0 "Quit" false)))

(fn ConstructionScript)